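; Behavior Tree task that stores the AI's own controlled BP_Unit in the SelfActor blackboard key.
; It scans every Unit actor in the level for the one whose AIController matches the task's owner, rather than reading the controlled pawn directly.
; It finishes successfully on a match, but has no failure path, so it never calls FinishExecute when no match is found.
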(event EventReceiveExecute
  (params (OwnerActor :type Actor%20Object%20Reference))
  (bind _outactors (Actor|GetAllActorsOfClass "/Script/ProjectSky.Unit"))
  (bind _array_element (Utilities|Array|ForEachLoopwithBreak _outactors)
    (:LoopBody
      (bind _asaicontroller (Utilities|Casting|CastToAIController OwnerActor))
      (bind _asaicontroller_2 (Utilities|Casting|CastToAIController (Pawn|GetController _array_element)))
      (if (== _asaicontroller_2 _asaicontroller)
        (bind _asbp_unit (Utilities|Casting|CastToBP_Unit _array_element))
        (Class|BTFunctionLibrary|SetBlackboardValueasObject (Variables|Default|GetSelfActor) _asbp_unit)
        (AI|BehaviorTree|FinishExecute true)))))