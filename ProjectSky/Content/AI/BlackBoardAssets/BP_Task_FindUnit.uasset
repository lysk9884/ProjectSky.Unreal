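; Behavior tree task that finds a nearby Unit from another squad for an AI-controlled Unit.
; It scans all Unit actors and compares each one's squad actor with that of the blackboard's SelfActor.
; The first Unit whose different squad actor lies within a fixed range, not necessarily the closest, is written to SelectedUnit along with its location.
; The task reports success after the loop even without a match.
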(event EventReceiveExecute
  (params (OwnerActor :type Actor%20Object%20Reference))
  (bind _outactors (Actor|GetAllActorsOfClass "/Script/ProjectSky.Unit"))
  (bind _array_element (Utilities|Array|ForEachLoopwithBreak _outactors :!label _label)
    (:LoopBody
      (bind _returnvalue (Class|Unit|GetSquadActor _array_element))
      (bind _asunit (Utilities|Casting|CastToUnit (Class|BTFunctionLibrary|GetBlackboardValueasObject (Variables|Default|GetSelfActor))))
      (bind _returnvalue_2 (Class|Unit|GetSquadActor _asunit))
      (if (!= _returnvalue_2 _returnvalue)
        (bind _returnvalue_3 (Transformation|GetDistanceTo _returnvalue_2 _returnvalue))
        (if (< _returnvalue_3 1e+03)
          (Class|BTFunctionLibrary|SetBlackboardValueasObject (Variables|Default|GetselectedUnit) _array_element)
          (AI|BehaviorTree|SetBlackboardValueasVector (Variables|Default|GetselectedUnitLocation) (Transformation|GetActorLocation _array_element))
          (goto _label Break))))
    (:Completed
      (AI|BehaviorTree|FinishExecute true))))