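; Behavior tree task that walks a BP_Unit toward its blackboard SelectedUnit, or to its squad formation slot when none is set.
; If the selected unit is within the mover's bounds Y extent, it stops that selected unit and succeeds.
; Otherwise it loops over all units, itself included, calling finish per element: failure and stopping the selected unit if one is that close, else moving and success.
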(event EventReceiveExecute
  (params (OwnerActor :type Actor%20Object%20Reference))
  (bind _asbp_unit (Utilities|Casting|CastToBP_Unit (AI|BehaviorTree|GetBlackboardValueasActor (Variables|Default|GetSelfActor))))
  (bind _asbp_unit_2 (Utilities|Casting|CastToBP_Unit (Class|BTFunctionLibrary|GetBlackboardValueasObject (Variables|Default|GetselectedUnit)))
    (:then
      (bind _returnvalue (Transformation|GetDistanceTo _asbp_unit _asbp_unit_2))
      (if (<= _returnvalue (.Y (Math|Vector|BreakVector (.BoxExtent (Collision|GetActorBounds _asbp_unit false)))))
        (Components|Movement|StopMovementImmediately _asbp_unit_2)
        (AI|BehaviorTree|FinishExecute true)
        (else
          (bind _outactors (Actor|GetAllActorsOfClass "/Game/Blueprints/Characters/BP_Unit.BP_Unit_C"))
          (bind _array_element (Utilities|Array|ForEachLoopwithBreak _outactors)
            (:LoopBody
              (bind _returnvalue_2 (Transformation|GetDistanceTo _array_element _asbp_unit))
              (if (<= _returnvalue_2 (.Y (Math|Vector|BreakVector (.BoxExtent (Collision|GetActorBounds _asbp_unit false)))))
                (Components|Movement|StopMovementImmediately _asbp_unit_2)
                (AI|BehaviorTree|FinishExecute false)
                (else
                  (Class|Unit|MovetoTargetPos _asbp_unit (Transformation|GetActorLocation _asbp_unit_2))
                  (AI|BehaviorTree|FinishExecute true))))))))
    (:CastFailed
      (bind _returnvalue_3 (Class|Unit|GetSquadActor _asbp_unit))
      (bind _assquad (Utilities|Casting|CastToSquad _returnvalue_3))
      (Class|Unit|MovetoTargetPos _asbp_unit (Class|Squad|GetUnitPos _assquad _asbp_unit (Class|UnitData|GetFormationIndex (Class|Unit|GetUnitData _asbp_unit))))
      (AI|BehaviorTree|FinishExecute true))))