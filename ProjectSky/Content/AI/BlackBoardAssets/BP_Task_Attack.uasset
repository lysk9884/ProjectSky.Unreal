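; Behavior tree task that makes an AI unit attack the unit stored in the SelectedUnit blackboard key.
; On execute it plays an attack montage on the SelfActor unit, then immediately applies fixed damage to the target's unit data if its HP is above zero.
; It finishes as failed without waiting for the montage, and never finishes if either BP_Unit cast fails.
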(event EventReceiveExecute
  (params (OwnerActor :type Actor%20Object%20Reference))
  (bind _asbp_unit (Utilities|Casting|CastToBP_Unit (AI|BehaviorTree|GetBlackboardValueasActor (Variables|Default|GetSelfActor))))
  (Animation|PlayAnimMontage _asbp_unit "/Game/Characters/DwarfGrunt/Anims/AnimMontageAttack_1_new.AnimMontageAttack_1_new" 1.0 "None")
  (bind _asbp_unit_2 (Utilities|Casting|CastToBP_Unit (Class|BTFunctionLibrary|GetBlackboardValueasObject (Variables|Default|GetselectedUnit))))
  (if (<= (Class|UnitData|GetCurrentHP (Class|Unit|GetUnitData _asbp_unit_2)) 0)
    _
    (else
      (Class|UnitData|AddHP (Class|Unit|GetUnitData _asbp_unit_2) -10)))
  (AI|BehaviorTree|FinishExecute false))