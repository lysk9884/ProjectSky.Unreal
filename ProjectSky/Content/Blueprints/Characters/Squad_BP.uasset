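; Squad pawn that groups BP_Unit members, can be initialized with a unit count, and is selected or deselected as a whole.
; InitSquad calls CreateSquad at the world origin and spawns a default controller.
; Selected has the passed controller possess and calls ToggleSelectionDecal(false) on every unit in MUnitPtrs, while Deselected passes true.
; GetPosition computes a line offset along X from unit index and actor scale.
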(event Custom|onUnitSelected
  (params (selectedUnit :type Controller%20Object%20Reference)))

(event EventSelected
  (params (Controller :type Controller%20Object%20Reference))
  (Pawn|Possess Controller)
  (for _array_element (Variables|Default|Getm_unitPtrs)
    (bind _asbp_unit (Utilities|Casting|CastToBP_Unit _array_element))
    (Default|ToggleSelectionDecal _asbp_unit false)))

(event EventDeselected
  (for _array_element (Variables|Default|Getm_unitPtrs)
    (bind _asbp_unit (Utilities|Casting|CastToBP_Unit _array_element))
    (Default|ToggleSelectionDecal _asbp_unit true)))

(fn ConstructionScript
  ;[1 1 1] initialiLize
)

(fn InitSquad
  (params (numUnit :type Integer))
  (bind _self self)
  (Class|Squad|CreateSquad _self numUnit "0, 0, 0")
  (Pawn|SpawnDefaultController _self))

(fn GetPosition
  (params (index :type Integer) (unitObj :type Actor%20Object%20Reference))
  (bind (_x _y _z) (Math|Vector|BreakVector "0, 0, 0"))
  (return (Math|Vector|MakeVector (+ _x (* (.X (Math|Vector|BreakVector (Transformation|GetActorScale3D unitObj))) (Math|Conversions|ToFloat(Integer) index))) _y _z)))