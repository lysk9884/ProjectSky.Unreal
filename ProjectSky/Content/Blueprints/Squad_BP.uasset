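; Squad actor Blueprint that represents a group of units, with unit-count limits and a world position set in its construction script.
; InitSquad delegates creation to CreateSquad, defined outside this file, then spawns a default controller for each unit in MUnitPtrs.
; An older BP_Fighter spawn path, including the GetPosition helper's X-axis spacing by actor scale, remains disconnected.
; The onUnitSelected event is empty.
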(event Custom|onUnitSelected
  (params (selectedUnit :type Controller%20Object%20Reference)))

(fn ConstructionScript
  ;[1 1 1] initialiLize
  (Variables|Default|Setm_maxUnitNum 3)
  (Variables|Default|Setm_minUnitNum 0)
  (Variables|Default|Setm_positon (Transformation|GetWorldLocation self)))

(fn InitSquad
  (params (numUnit :type Integer))
  (Class|Squad|CreateSquad self numUnit)
  (for _array_element (Variables|Default|Getm_unitPtrs)
    (Pawn|SpawnDefaultController _array_element)))

(fn GetPosition
  (params (index :type Integer) (unitObj :type Actor%20Object%20Reference))
  (bind _m_positon (Variables|Default|Getm_positon))
  (bind (_x _y _z) (Math|Vector|BreakVector _m_positon))
  (return (Math|Vector|MakeVector (+ _x (* (.X (Math|Vector|BreakVector (Transformation|GetActorScale3D unitObj))) (Math|Conversions|ToFloat(Integer) index))) _y _z)))