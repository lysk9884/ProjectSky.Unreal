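; BP_RTS_GameState is the game state for an RTS, holding the shared Wood, Gold and Food resource totals.
; Three events, UpdateWood, UpdateGold and UpdateFood, each add a given amount to the matching total.
; The totals are not clamped or checked, and the events neither notify listeners nor contain other logic.
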(event Custom|UpdateWood
  (params (Amount :type Integer))
  (Variables|Default|SetWood (+ (Variables|Default|GetWood) Amount)))

(event Custom|UpdateGold
  (params (Amount :type Integer))
  (Variables|Default|SetGold (+ (Variables|Default|GetGold) Amount)))

(event Custom|UpdateFood
  (params (Amount :type Integer))
  (Variables|Default|SetFood (+ (Variables|Default|GetFood) Amount)))

(fn ConstructionScript)